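; Base weapon actor for a shooter that fires hitscan shots, spending ammo and playing muzzle effects.
; Automatic fire opens a Tick-driven Gate while single fire triggers once, both throttled by a DoOnce that resets after the FireRate delay.
; Shots trace from the owner's camera along control rotation, spawning impact effects and damaging any BP_ShooterCharacter hit.
; UpdateValues loads stats and effects from DT_Weapon by WeaponID, and Ammo's RepNotify broadcasts changes through a dispatcher.
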(event Custom|Play%20Impact%20Effect
  (params (HitResult :type Hit%20Result%20Structure))
  (bind _location (Collision|BreakHitResult HitResult))
  ;[1 1 1] Play Impact Effects
  (Niagara|SpawnSystematLocation (Variables|Effect|GetNiagara%20Impact%20Effect) _location)
  (Audio|SpawnSoundatLocation (Variables|Effect|GetHit%20Sound) _location "0, 0, 0" 1.0 1.0 0.0 0 0))

(event Custom|Event%20Fire%20Off
  (Utilities|FlowControl|Gate true) ; enters at Close
)

(event Custom|Event%20Shake%20Camera
  ;[1 1 1] Shake Camera
  (CameraShakes|StartCameraShake (Game|GetPlayerCameraManager 0) (Variables|CameraShake|GetCamera%20Shake) (Variables|CameraShake|GetCamera_Shake_Scale) "CameraLocal" "0, 0, 0"))

(event Custom|Fire
  (if (CallFunction|IsEnoughAmmo)
    (CallFunction|DecreaseAmmo)
    (CallFunction|CauseDamage)
    (Audio|PlaySoundatLocation (Variables|Effect|GetMuzzle%20Sound) (Transformation|GetActorLocation) "0, 0, 0" 1.0 1.0 0.0 0 0 0 0)
    (Niagara|SpawnSystemAttached (Variables|Effect|GetProjectile%20Muzzle%20Flash) (Variables|Default|GetMuzzle%20Flash%20Location) "None" "0, 0, 0" "0.000000,90.000000,0.000000" "KeepRelativeOffset" true)))

(event Custom|Cause%20Damage
  (bind _returnvalue (Components|GetOwner))
  (bind _returnvalue_2 (Actor|GetComponentbyClass _returnvalue "/Script/Engine.CameraComponent"))
  (bind _returnvalue_3 (Transformation|GetWorldLocation _returnvalue_2))
  (bind (_outhit _returnvalue_4) (Collision|LineTraceByChannel _returnvalue_3 (+ _returnvalue_3 (* (Math|Rotator|GetRotationXVector (Pawn|GetControlRotation (Game|GetInstigatorController _returnvalue) :!class /Script/Engine.Controller)) (Variables|Basic|GetRange))) "TraceTypeQuery3" false 0 "ForDuration"))
  (if _returnvalue_4
    (CallFunction|PlayImpactEffect _outhit)
    (bind _asbp_shooter_character (Utilities|Casting|CastToBP_ShooterCharacter (.HitActor (Collision|BreakHitResult _outhit))))
    (Class|IDamage|GetDamage _asbp_shooter_character (Variables|Basic|GetDamage))))

(event Custom|Reload%20Ammo
  (Variables|Default|SetAmmo (Variables|Basic|GetMax%20Ammo)))

(event Custom|Event%20Fire%20On
  (if (Variables|Basic|GetIsAutomatic)
    (Utilities|FlowControl|Gate true) ; enters at Open
    (else
      (Utilities|FlowControl|DoOnce false :!label _label
        (:Completed
          (CallFunction|Fire)
          (Utilities|FlowControl|Delay (Variables|Default|GetFire%20Rate))
          (goto _label Reset))))))

(event EventTick
  (params (DeltaSeconds :type Float%20%28single-precision%29))
  (Utilities|FlowControl|Gate true
    (:Exit
      (Utilities|FlowControl|DoOnce false :!label _label
        (:Completed
          (CallFunction|Fire)
          (Utilities|FlowControl|Delay (Variables|Default|GetFire%20Rate))
          (goto _label Reset))))))

(fn ConstructionScript
  (Variables|Default|SetAmmo (Variables|Basic|GetMax%20Ammo)))

(fn IsEnoughAmmo
  (return (> (Variables|Default|GetAmmo) 0)))

(fn DecreaseAmmo
  (Variables|Default|SetAmmo (- (Variables|Default|GetAmmo) 1)))

(fn OnRepAmmo
  (CallFunction|UpdateAmmo))

(fn UpdateAmmo
  (Default|CallEDAmmoChanged (Variables|Default|GetAmmo)))

(fn UpdateValues
  (bind _returnvalue (Utilities|GetDataTableRow "/Game/DataTable/DT_Weapon.DT_Weapon" (Variables|Default|GetWeapon%20ID))
    (:then
      (Variables|Basic|SetIsAutomatic (.isAutomatic (Utilities|Struct|BreakS_Weapon _returnvalue)))
      (Variables|Basic|SetMax%20Ammo (.Ammo (Utilities|Struct|BreakS_Weapon _returnvalue)))
      (Variables|Default|SetFire%20Rate (.FireRate (Utilities|Struct|BreakS_Weapon _returnvalue)))
      (Variables|Basic|SetDamage (.Damage (Utilities|Struct|BreakS_Weapon _returnvalue)))
      (Variables|Effect|SetProjectile%20Muzzle%20Flash (.MuzzleEffect (Utilities|Struct|BreakS_Weapon _returnvalue)))
      (Variables|Effect|SetNiagara%20Impact%20Effect (.ImpactEffect (Utilities|Struct|BreakS_Weapon _returnvalue)))
      (Variables|Effect|SetHit%20Sound (.ImpactSound (Utilities|Struct|BreakS_Weapon _returnvalue)))
      (Variables|Effect|SetMuzzle%20Sound (.MuzzleSound (Utilities|Struct|BreakS_Weapon _returnvalue))))))