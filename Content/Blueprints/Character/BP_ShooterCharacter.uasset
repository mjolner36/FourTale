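; BP_ShooterCharacter is a networked shooter character that owns an automatic weapon, takes damage and respawns through the game mode.
; It spawns BP_WeaponAuto onto a hand mesh socket, passes fire input through server and multicast events, and broadcasts weapon changes via OnRep.
; Damage feeds the Health component, whose death event removes the HUD and triggers a delayed respawn.
; Local-controller checks gate HUD drawing, and a head-bob camera shake event covers movement.
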(event Custom|Event%20Add%20Weapon
  (bind _returnvalue (Game|SpawnActorfromClass "/Game/Blueprints/Gun/BP_WeaponAuto.BP_WeaponAuto_C" (Transformation|GetSocketTransform (Variables|Character|GetMesh) "WeaponSocket" "RTS_World") "AlwaysSpawn" self 0))
  (bind _output_get (Variables|Default|SetWeapon _returnvalue))
  (Transformation|AttachComponentToComponent _output_get (Variables|Character|GetMesh) "WeaponSocket" "SnapToTarget" "SnapToTarget" "SnapToTarget" true)
  (Default|UpdateValues _output_get))

(event Custom|Event%20On%20Died
  (Variables|Default|SetIs%20Dead true)
  (CallFunction|OwnUIDelete)
  (Utilities|FlowControl|Delay 3.0)
  (Default|Respawn (CallFunction|FLGetGameMode) (Game|GetInstigatorController)))

(event Custom|Own%20UI%20Delete
  (if (CallFunction|IsLocalController)
    (Default|DeleteUI (CallFunction|GetPlayerHUD (Pawn|GetController)))))

(event Custom|Own%20UI%20Draw
  ;[1 1 1] Draw UI
  (if (CallFunction|IsLocalController)
    (Default|DrawUI (CallFunction|GetPlayerHUD (Pawn|GetController)))))

(event Custom|Fire%20Multi
  (params (Can%20Fire :type Boolean))
  (bind _weapon (Variables|Default|GetWeapon))
  ;[1 1 1] Fire Weapon
  (if Can%20Fire
    (Default|EventFireon _weapon)
    (else
      (Default|EventFireOff _weapon))))

(event Custom|Fire%20Server
  (params (Can%20Fire :type Boolean))
  ;[1 1 1] Fire Weapon
  (CallFunction|FireMulti Can%20Fire))

(event EventBeginPlay
  ;[0.5914 0.576 1] Init
  (|CallParentFunction)
  (EventDispatchers|AssignOnDied (Variables|Default|GetHealth) (delegate Custom|Event%20On%20Died))
  (CallFunction|EventAddWeapon))

(event EventPossessed
  (params (NewController :type Controller%20Object%20Reference))
  ;[1 1 1] Draw UI
  (Utilities|FlowControl|Delay 1.0)
  (CallFunction|OwnUIDraw))

(event EventGetDamage
  (params (Damage :type Float%20%28single-precision%29))
  (Class|HealthComponent|TakeDamage (Variables|Default|GetHealth) Damage))

(event EventCameraShakeonMove
  (CameraShakes|StartCameraShake (Game|GetPlayerCameraManager 0) "/Game/Blueprints/CameraShake/CamShake_HeadBob_Walking.CamShake_HeadBob_Walking_C" 0.5 "CameraLocal" "0, 0, 0"))

(event Input|ActionEvents|InputActionReload
  (params (Key :type Key%20Structure :default "None"))
  ;[1 1 1] Reload
  (:Pressed
    (Default|ReloadAmmo (Variables|Default|GetWeapon))))

(event Input|ActionEvents|InputActionShoot
  (params (Key :type Key%20Structure :default "None"))
  (:Pressed
    (CallFunction|FireServer true))
  (:Released
    (CallFunction|FireServer false)))

(fn ConstructionScript)

(fn OnRepWeapon
  (Default|CallEDWeaponChanged))

(fn GetPlayerHUD
  (params (Object :type Controller%20Object%20Reference))
  (bind _asplayer_controller (Utilities|Casting|CastToPlayerController Object))
  (bind _ashud_game (Utilities|Casting|CastToHUD_Game (HUD|GetHUD _asplayer_controller)))
  (return _ashud_game))

(fn IsLocalController
  (return (Pawn|IsLocalController (Pawn|GetController))))