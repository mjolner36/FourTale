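; GS_ShooterV2, by its name the shooter's game state, holds the match time left in seconds and shows it on the player HUD.
; On BeginPlay it caches player 0's HUD as HUD_Game.
; UpdateHUDMacthTimer sets the RepNotify time variable, whose OnRep passes the value to the HUD's PlayerUI through UpdateTime when both references are valid.
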(event Custom|Update%20HUD%20Macth%20Timer
  (params (Mach%20Time%20Left%20Sec :type Integer))
  (Variables|Default|SetMach%20Time%20Left%20Sec Mach%20Time%20Left%20Sec))

(event EventBeginPlay
  (bind _ashud_game (Utilities|Casting|CastToHUD_Game (HUD|GetHUD (Game|GetPlayerController 0))))
  (Variables|Default|SetPlayer%20HUD%20Game%20Ref _ashud_game))

(fn ConstructionScript)

(fn OnRepMachTimeLeftSec
  (bind _player_hud_game_ref (Variables|Default|GetPlayer%20HUD%20Game%20Ref)
    (:then
      (bind _player_ui (Variables|/Game/UI/HUD_Game.HUD_Game_C|GetPlayer%20UI _player_hud_game_ref)
        (:then
          (Default|UpdateTime _player_ui (Variables|Default|GetMach%20Time%20Left%20Sec)))
        (:else)))
    (:else)))